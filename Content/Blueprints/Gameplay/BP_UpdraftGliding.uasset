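; Updraft volume that boosts a gliding main character upward when they enter its capsule.
; On overlap it calls the character's Glide and launches it with a Z-override velocity, using a DoOnce that resets after the character's max glide time.
; The construction script scales a capless cylinder mesh vertically to match the capsule's straight section, converting centimetres to metres.
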(event `self.Capsule.OnComponentBeginOverlap`
  (params (OverlappedComponent :type "PrimitiveComponent Object Reference") (OtherActor :type "Actor Object Reference") (OtherComp :type "PrimitiveComponent Object Reference") (OtherBodyIndex :type Integer) (bFromSweep :type Boolean) (SweepResult :type "HitResult Structure (by ref)"))
  (bind _asbp_main_character (cast `/Game/Blueprints/Characters/BP_MainCharacter` OtherActor))
  (if (`/Game/Blueprints/Characters/BP_MainCharacter.isGliding` _asbp_main_character)
    (`/Engine/EditorBlueprintResources/StandardMacros.DoOnce` false :!label _label
      (:`Completed`
        (`KismetSystemLibrary.PrintString` "Updraft" true true (struct :`R` 0.946028 :`G` 1.0 :`B` 0.212663 :`A` 1.0))
        (`/Game/Blueprints/Characters/BP_MainCharacter.Glide` _asbp_main_character)
        (`Character.LaunchCharacter` _asbp_main_character (`KismetMathLibrary.MakeVector` 0.0 0.0 (`self.Launch Velocity Z`)) false true)
        (`KismetSystemLibrary.Delay` (`/Game/Blueprints/Characters/BP_MainCharacter.MaxGlideTime` _asbp_main_character))
        (goto _label :!via `Reset`)))))

(fn `UserConstructionScript`
  (`SceneComponent.SetRelativeScale3D` (`self.Cylinder1mNoCap`) (`KismetMathLibrary.MakeVector` 1.0 1.0 (/ (* (- (`CapsuleComponent.CapsuleHalfHeight` (`self.Capsule`)) 100.0) 2.0) 100.0))))
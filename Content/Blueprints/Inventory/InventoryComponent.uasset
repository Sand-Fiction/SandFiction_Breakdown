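; Inventory component that stores items in a list and tracks which ones have been gifted.
; Adding resolves a data table row handle, appends the row with AddUnique and prints whether it was added or already held.
; Gifting rebuilds the item struct without the gifted flag to find an ungifted match, then overwrites it as gifted and returns true, or prints a failure and returns false.
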(fn `AddItemToInventory`
  (params (ItemData :type "DataTableRowHandle Structure"))
  (bind (_datatable _rowname) (break `DataTableRowHandle` ItemData))
  (bind _returnvalue (`|GetDataTableRow` _datatable _rowname)
    (:`then`
      (bind _returnvalue_2 (`KismetArrayLibrary.Array_AddUnique` (`self.ItemList`) _returnvalue))
      (if (!= _returnvalue_2 -1)
        (bind _name (break `/Game/Blueprints/Inventory/ItemStructure` _returnvalue))
        (`KismetSystemLibrary.PrintString` (`KismetTextLibrary.Conv_TextToString` (`|FormatText` "{Name} added to Inventory" _name)))
        (else
          (`KismetSystemLibrary.PrintString` (`KismetTextLibrary.Conv_TextToString` (`|FormatText` "{Name} is already in Inventory" _name))))))))

(fn `SetItemGifted`
  (params (ItemData :type "DataTableRowHandle Structure"))
  (returns (Success :type Boolean))
  (bind (_datatable _rowname) (break `DataTableRowHandle` ItemData))
  (bind _itemlist (`self.ItemList`))
  (bind _returnvalue (`|GetDataTableRow` _datatable _rowname)
    (:`then`
      (bind (_name _icon _description) (break `/Game/Blueprints/Inventory/ItemStructure` _returnvalue))
      (bind _itemstructure (make `/Game/Blueprints/Inventory/ItemStructure` _name _icon _description false (struct :`RowName` "Default")))
      (bind _returnvalue_2 (`KismetArrayLibrary.Array_Find` _itemlist _itemstructure))
      (if (!= _returnvalue_2 -1)
        (bind (_name_2 _icon_2 _description_2) (break `/Game/Blueprints/Inventory/ItemStructure` _itemstructure))
        (`KismetArrayLibrary.Array_Set` _itemlist _returnvalue_2 (make `/Game/Blueprints/Inventory/ItemStructure` _name_2 _icon_2 _description_2 true (struct :`RowName` "Default")))
        (return true)
        (else
          (`KismetSystemLibrary.PrintString` " Item cannot be gifted, because it's not in Inventory or it's already gifted." true true (struct :`R` 1.0 :`B` 0.040611 :`A` 1.0))
          (return false))))))
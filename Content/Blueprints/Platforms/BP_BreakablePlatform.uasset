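; Breakable platform that changes color and shatters some time after the main character hits it.
; A hit on the Destructible stores the impact point and plays a timeline, rate-scaled by TimeUntilBreak, that drives a dynamic material's color.
; When the timeline finishes, the mesh simulates physics, takes radial damage with an impulse at that point, and the actor is destroyed after a delay.
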(event `self.Destructible.OnComponentHit`
  (params (HitComponent :type "PrimitiveComponent Object Reference") (OtherActor :type "Actor Object Reference") (OtherComp :type "PrimitiveComponent Object Reference") (NormalImpulse :type "Vector Structure") (Hit :type "HitResult Structure (by ref)"))
  (cast `/Game/Blueprints/Characters/BP_MainCharacter` OtherActor
    (:`then`
      (set `self.Hit Location` (`.Location` (`GameplayStatics.BreakHitResult` Hit)))
      (`TimelineComponent.Play` (`self.TimeUntilDestroy`)))
    (:`CastFailed`
      (`KismetSystemLibrary.PrintString` "Not MC somehow dunno LOL"))))

(fn `UserConstructionScript`
  (`parent.UserConstructionScript`)
  (bind _returnvalue (`PrimitiveComponent.CreateDynamicMaterialInstance` (`self.Destructible`) 0 "/Game/Materials/M_ColorableShape.M_ColorableShape" "None"))
  (bind _output_get (set `self.Material` _returnvalue))
  (`PrimitiveComponent.SetMaterial` (`self.Destructible`) 0 _output_get)
  (`TimelineComponent.SetPlayRate` (`self.TimeUntilDestroy`) (/ 1.0 (`self.TimeUntilBreak`))))
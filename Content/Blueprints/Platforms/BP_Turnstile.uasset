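; BP_Turnstile is a platform Blueprint that turns around its yaw axis when its Trigger event fires.
; A DoOnce gate lets the trigger through, caches the root's world rotation and plays the Rotation timeline from the start.
; The timeline adds its value to the cached yaw each update.
; On finish, the gate resets only if RotationLoop is set, allowing another trigger to turn it further.
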(event `self.Trigger`
  (bind (_current_rotation_roll _current_rotation_pitch _current_rotation_yaw) (`KismetMathLibrary.BreakRotator` (`self.Current Rotation`)))
  (`/Engine/EditorBlueprintResources/StandardMacros.DoOnce` false :!label _label
    (:`Completed`
      (set `self.Current Rotation` (`SceneComponent.K2_GetComponentRotation` (`self.Root`)))
      (bind (_direction _rotation) (`Timeline|Rotation` :!via `PlayFromStart`)
        (:`Update`
          (`SceneComponent.K2_SetWorldRotation` (`self.Root`) (`KismetMathLibrary.MakeRotator` _current_rotation_roll _current_rotation_pitch (+ _current_rotation_yaw _rotation)) false false))
        (:`Finished`
          (if (`self.RotationLoop`)
            (goto _label :!via `Reset`)))))))

(fn `UserConstructionScript`
  (`parent.UserConstructionScript`))
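; BP_Doorway is a platform doorway that a player triggers to open or close, optionally gated by Energy Cores.
; A positive EnergyThreshold checks the player's InventoryComponent without deducting cores, printing a message with a hardcoded count of 3 on failure.
; An ActorSequence plays forward or in reverse according to the Closed flag.
; A DoOnce limits this to one toggle, resetting afterward only when Closable is set.
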(event `self.Trigger`
  (params (Player :type "/Game/Blueprints/Characters/BP_MainCharacter Object Reference"))
  (bind _sequenceplayer (`ActorSequenceComponent.SequencePlayer` (`self.ActorSequence`)))
  (if (> (`self.EnergyThreshold`) 0)
    (if (>= (`/Game/Blueprints/Inventory/InventoryComponent.EnergyCore` (`/Game/Blueprints/Characters/BP_MainCharacter.InventoryComponent` Player)) (`self.EnergyThreshold`))
      (`/Engine/EditorBlueprintResources/StandardMacros.DoOnce` false :!label _label
        (:`Completed`
          (if (`self.Closed`)
            (`MovieSceneSequencePlayer.Play` _sequenceplayer)
            (set `self.Closed` false)
            (else
              (`MovieSceneSequencePlayer.PlayReverse` _sequenceplayer)
              (set `self.Closed` true)))
          (if (`self.Closable`)
            (goto _label :!via `Reset`))))
      (else
        (`KismetSystemLibrary.PrintString` "Not enough Energy Cores! Need: 3")))
    (else
      (goto _label))))

(fn `UserConstructionScript`
  (`parent.UserConstructionScript`))